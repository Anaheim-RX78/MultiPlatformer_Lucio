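; BP_Button is a pressure button that the third-person character presses by overlapping its ActuatorCollider.
; Overlap plays a Timeline that moves the Actuator along Z, and ending the overlap reverses it.
; When the Timeline finishes, its direction decides whether the ActivateButton or DeactivateButton dispatcher is called, so each fires only after the movement completes.
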(event `self.ReceiveBeginPlay`)

(event `self.ActuatorCollider.OnComponentBeginOverlap`
  (params (OverlappedComponent :type "PrimitiveComponent Object Reference") (OtherActor :type "Actor Object Reference") (OtherComp :type "PrimitiveComponent Object Reference") (OtherBodyIndex :type Integer) (bFromSweep :type Boolean) (SweepResult :type "HitResult Structure (by ref)"))
  (cast `/Game/ThirdPerson/Blueprints/BP_ThirdPersonCharacter` OtherActor)
  (bind (_direction _newtrack_0) (`Timeline|Timeline` :!label _label)
    (:`Update`
      (`SceneComponent.K2_SetRelativeLocation` (`self.Actuator`) (`KismetMathLibrary.MakeVector` 0.0 0.0 (* _newtrack_0 -10.0)) false false))
    (:`Finished`
      (if (`|EnumEquality` _direction "Forward")
        (`self.ActivateButton`)
        (else
          (`self.DeactivateButton`))))))

(event `self.ActuatorCollider.OnComponentEndOverlap`
  (params (OverlappedComponent :type "PrimitiveComponent Object Reference") (OtherActor :type "Actor Object Reference") (OtherComp :type "PrimitiveComponent Object Reference") (OtherBodyIndex :type Integer))
  (cast `/Game/ThirdPerson/Blueprints/BP_ThirdPersonCharacter` OtherActor)
  (goto _label :!via `Reverse`))

(fn `UserConstructionScript`)